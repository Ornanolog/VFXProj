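; AfterimageBP is an afterimage actor that mirrors another skeletal mesh's pose on a poseable mesh with an animated positional offset.
; Every Tick copies the pose from RefPose and calls Play on a timeline.
; The timeline's X and Z outputs, scaled down and multiplied by Mult, nudge the mesh's relative location cumulatively.
; On finishing, the timeline restarts in its current direction, so the motion loops.
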(event EventBeginPlay)

(event Collision|EventActorBeginOverlap
  (params (OtherActor :type Actor%20Object%20Reference)))

(event EventTick
  (params (DeltaSeconds :type Float%20%28single-precision%29))
  (bind _mult (Variables|Default|GetMult))
  (Class|PoseableMeshComponent|CopyPosefromSkeletalComponent (Variables|Default|GetPoseableMesh) (Variables|Default|GetRefPose))
  (bind (_direction _x _z) (Timeline|Timeline_0 Play)
    (:Update
      (Transformation|AddRelativeLocation (Variables|Default|GetPoseableMesh) (Math|Vector|MakeVector (* (/ _x 5.0) _mult) 0.0 (* (/ _z 5.0) _mult)) false false))
    (:Finished
      (switch Utilities|FlowControl|Switch|SwitchonETimelineDirection _direction
        (:Forward
          (Timeline|Timeline_0 PlayFromStart))
        (:Backward
          (Timeline|Timeline_0 ReverseFromEnd))))))

(fn ConstructionScript)