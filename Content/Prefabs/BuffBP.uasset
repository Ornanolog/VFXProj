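; BuffBP is an actor that plays a scripted shield buff sequence on its skeletal mesh at BeginPlay.
; The buff animation starts with a leaf Niagara burst, then after a delay an AfterimageBP spawns from the mesh and a shield effect attaches to the pelvis.
; An Emissive timeline drives the ShieldParameters collection's Blackbody value and refreshes the afterimage's reference mesh.
; A delay chained to the timeline's updates returns the mesh to looping idle.
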(event EventBeginPlay
  (bind _skeletalmesh (Variables|Default|GetSkeletalMesh))
  (bind _returnvalue (Transformation|GetWorldTransform _skeletalmesh))
  (Components|Animation|PlayAnimation _skeletalmesh "/Game/MagicalAnim/Animations/attack/10_buff/10_buff.10_buff" false)
  (Niagara|SpawnSystematLocation "/Game/Particles/NS_ShieldLeaves.NS_ShieldLeaves" (Math|Transform|TransformLocation _returnvalue "0, 0, 0"))
  (Utilities|FlowControl|Delay 2.36)
  (bind _returnvalue_2 (Game|SpawnActorfromClass "/Game/Prefabs/AfterimageBP.AfterimageBP_C" _returnvalue "Undefined" 0 _skeletalmesh 0.0 0.3 0))
  (Niagara|SpawnSystemAttached "/Game/Particles/NS_Shield.NS_Shield" _skeletalmesh "pelvis" "-20.000000,0.000000,0.000000" "90.000000,-20.000000, 0" "KeepRelativeOffset" false)
  (bind _newtrack_0 (Timeline|Emissive Play)
    (:Update
      (Rendering|Material|SetScalarParameterValue "/Game/Materials/ShieldParameters.ShieldParameters" "Blackbody" _newtrack_0 :!class /Script/Engine.KismetMaterialLibrary)
      (Variables|/Game/Prefabs/AfterimageBP.AfterimageBP_C|SetRefPose _returnvalue_2 _skeletalmesh)
      (Utilities|FlowControl|Delay 2.8)
      (Components|Animation|PlayAnimation _skeletalmesh "/Game/MagicalAnim/Animations/idle/01_idle.01_idle" true))))

(event EventTick
  (params (DeltaSeconds :type Float%20%28single-precision%29)))

(fn ConstructionScript)